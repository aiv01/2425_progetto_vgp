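; Road spline actor for the procedural dressing tool's PCG setup, with all its logic in the Construction Script.
; It stores the chosen Mesh as a soft object path in MeshPath.
; It rebuilds Spline1 as a hidden copy of Spline, point by point, copying locations in local space and rotations and tangents in world space.
; The event graph holds no active logic.
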(event EventBeginPlay)

(event Collision|EventActorBeginOverlap
  (params (OtherActor :type Actor%20Object%20Reference)))

(event EventTick
  (params (DeltaSeconds :type Float%20%28single-precision%29)))

(fn ConstructionScript
  (bind _spline (Variables|Default|GetSpline))
  (bind _spline1 (Variables|Default|GetSpline1))
  (Variables|Variables|SetMeshPath (Utilities|GetSoftObjectPath (Variables|Default|GetMesh)))
  (bind _output_get (Variables|Default|SetNewVar (Spline|GetNumberOfSplinePoints (Variables|Default|GetSpline))))
  (Spline|ClearSplinePoints (Variables|Default|GetSpline1) true)
  (for _index (range 0 (- _output_get 1))
    (Variables|Default|SetIndex _index)
    (Spline|AddSplinePointatIndex _spline1 (Spline|GetLocationatSplinePoint _spline (Variables|Default|GetIndex) "Local") (Variables|Default|GetIndex) "Local" true)
    (Spline|SetRotationatSplinePoint _spline1 (Variables|Default|GetIndex) (Spline|GetRotationatSplinePoint _spline (Variables|Default|GetIndex) "World") "World" true)
    (Spline|SetTangentsatSplinePoint _spline1 (Variables|Default|GetIndex) (.arrivetangent (Spline|GetSplinePointAt _spline (Variables|Default|GetIndex) "World")) (.leavetangent (Spline|GetSplinePointAt _spline (Variables|Default|GetIndex) "World")) "World" true)
    (Rendering|SetVisibility _spline1 false false)))