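; BP_WaveManagerTester is a debug harness for exercising a wave manager.
; On BeginPlay it binds to the manager's enemy spawn, enemy death, wave start, wave completion and level end events, printing each to screen.
; StartWaveSystem starts the manager unless it is set to auto-start.
; StartKillEnemies simulates kills by calling StaticHandleEnemyDie with itself on a configurable, optionally looping timer.
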(event Custom|Start%20Kill%20Enemies
  (Utilities|Time|SetTimerbyEvent (delegate Custom|DieEnemy) (Variables|Default|GetFrequencyEnemyKill) (Variables|Default|GetLoopingEnemyKill)))

(event Custom|DieEnemy
  (Class|PWaveManager|StaticHandleEnemyDie self))

(event Custom|StartWaveSystem
  (bind _wavemngr (Variables|Default|GetWaveMngr))
  (if (not (Variables|/Script/WaveTool.PWaveManager|GetbAutoStartWaveSystem _wavemngr))
    (Class|PWaveManager|StartWaveSystem _wavemngr)
    (else
      (Development|PrintString "WaveSystemAlreadyStarted"))))

(event EventBeginPlay
  (|BindingEventWaveManager))

(fn ConstructionScript)

(event Custom|OnEndLevel
  (Development|PrintString "EndLevel"))

(event Custom|OnEnemyDie
  (params (EnemyDie :type Actor%20Object%20Reference))
  (Development|PrintString (Utilities|String|Append "EnemyDie: " (Utilities|GetDisplayName EnemyDie))))

(event Custom|OnWaveCompleted
  (params (WaveIndex :type Integer))
  (Development|PrintString (Utilities|String|Append "WaveCompleted: " (Utilities|String|ToString(Integer) WaveIndex))))

(event Custom|OnWaveStarted
  (params (WaveIndex :type Integer))
  (Development|PrintString (Utilities|String|Append "WaveStarted: " (Utilities|String|ToString(Integer) WaveIndex))))

(event Custom|OnEnemySpawn
  (params (EnemySpawn :type Actor%20Object%20Reference))
  (Development|PrintString (Utilities|String|Append "EnemySpawned: " (Utilities|GetDisplayName EnemySpawn))))