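; GOAP-driven enemy character that can lead or follow in a formation.
; A GOAP component chooses goals from world-state updates, while AbilitySystem runs skill strategies, currently a hardcoded "Test".
; On spawn info, leaders get a speed multiplier; followers add a follow-slot action and claim the leader's first free slot.
; Interface functions expose players, spline path, nexus and slot position, computed relative to the leader's transform from DataTable-defined offsets.
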(event EventBeginPlay
  ;[1 0.4146 0] Play Skill with name event name (Hypotesis: Map<Name, Function>)
  (bind _values (Utilities|Map|Values (Variables|/Script/AIV_2025_VGP.AbilitySystemComponent|GetStrategyInstances (Variables|Default|GetAbilitySystem))))
  (for _array_element _values
    (Variables|/Script/AIV_2025_VGP.GOAPBaseStrategy|SetStrategyOwner _array_element self)))

(event EventUpdateWorldState
  (params (wd :type GOAP%20World%20Model%20Object%20Reference))
  (Default|ChoseGoal (Variables|Default|GetGOAP) wd))

(event EventIExecuteSkill
  (params (SkillName :type Name :default "None"))
  ;[1 0.4146 0] Play Skill with name event name (Hypotesis: Map<Name, Function>)
  (Class|AbilitySystemComponent|ExecuteStrategy (Variables|Default|GetAbilitySystem) "Test"))

(event EventSetSpawnInfo
  (params (bIsLeader :type Boolean) (FormationName :type Name :default "None") (GroupID :type Integer))
  ;[1 1 1] Spawn
  (CallFunction|SpawnInfoInitialization bIsLeader FormationName GroupID)
  (Development|PrintString "è andata"))

(event Custom|Init%20GOAP
  (Default|InitializeGOAP (Variables|Default|GetGOAP)))

(fn ConstructionScript
  (|CallParentFunction))

(fn IGetPlayers
  (Utilities|Array|Add (Variables|TEMP_WorldLinker|GetPlayers) (Game|Player|GetPlayerPawn 0))
  (return (Variables|TEMP_WorldLinker|GetPlayers)))

(fn IFindNearestPlayer
  (for _array_element (Variables|TEMP_WorldLinker|GetPlayers)
    (if (and true (> (LocalVariables|GetCurrent%20Min%20Distance) (Class|KismetMathLibrary|VectorDistanceSquared (Transformation|GetActorLocation _array_element) (Transformation|GetActorLocation))))
      (LocalVariables|SetCurrent%20Min%20Distance (Class|KismetMathLibrary|VectorDistanceSquared (Transformation|GetActorLocation _array_element) (Transformation|GetActorLocation)))
      (LocalVariables|SetNearest%20P _array_element)))
  (return (LocalVariables|GetNearest%20P)))

(fn IGetSplinetoFollow
  (return (Variables|Default|GetSpline%20Path)))

(fn IGetNexus
  (return (Variables|TEMPWorldLinker|GetNexus)))

(fn InitAI)

(fn SpawnInfoInitialization
  (params (New%20Is%20Leader :type Boolean) (New%20Formation%20Name :type Name) (New%20Group%20ID :type Integer))
  (Variables|FormationLeader|SetIs%20Leader New%20Is%20Leader)
  (Variables|FormationLeader|SetFormation%20Name New%20Formation%20Name)
  (Variables|FormationLeader|SetGroup%20ID New%20Group%20ID)
  (if (Variables|FormationLeader|GetIs%20Leader)
    (Variables|/Script/Engine.CharacterMovementComponent|SetMaxWalkSpeed (Variables|Character|GetCharacterMovement) (* (Variables|FormationLeader|GetFormation%20Leader%20Speed%20Mult) (Variables|/Script/Engine.CharacterMovementComponent|GetMaxWalkSpeed (Variables|Character|GetCharacterMovement))))
    (else
      (Utilities|FlowControl|Sequence
        (:then_0
          ;[1 1 1] GOAP Action
          (bind _returnvalue (Game|ConstructObjectfromClass "/Game/Custom/Characters/Enemies/Components/GOAP/Actions/MovementAction/BP_GOAPA_FollowFormationSlot.BP_GOAPA_FollowFormationSlot_C" (Variables|FormationElement|GetFormation%20Pos%20Acceptance%20Radius)))
          (Utilities|Map|Add (Variables|/Script/AIV_2025_VGP.GOAPAction|GetSatisfiers _returnvalue) "RespectFormation" (Variables|FormationElement|GetRespect%20Formation%20Satisfaction))
          (Variables|/Script/AIV_2025_VGP.GOAPAction|SetExecuter _returnvalue self)
          (Utilities|Array|AddUnique (Variables|/Script/AIV_2025_VGP.GOAPAgentComponent|GetActions (Variables|Default|GetGOAP)) _returnvalue))
        (:then_1
          (Formation|BindFormationElement (Variables|FormationElement|GetLeader%20Ref) self))))))

(fn SetupFormationPositions
  (params (Formation%20Name :type Name))
  (bind _returnvalue (Utilities|GetDataTableRow "/Game/Custom/Characters/Enemies/ConcreteEnemies/Formation/DT_Formations.DT_Formations" Formation%20Name)
    (:then
      (for _array_element (.positions _returnvalue)
        (Utilities|Array|Add (Variables|FormationLeader|GetFormation%20Points) (Utilities|Struct|MakeS_FormationSlot 0 _array_element))))))

(fn BindFormationElement
  (params (Former%20Element :type BP%20Goap%20Agent%20Object%20Reference))
  (bind (_array_element _array_index) (Utilities|Array|ForEachLoopwithBreak (Variables|FormationLeader|GetFormation%20Points) :!label _label)
    (:LoopBody
      (Utilities|IsValid (.occupier _array_element)
        (:Is%20Not%20Valid
          (Utilities|Struct|SetmembersinS_FormationSlot (Utilities|Array|Get(acopy) (Variables|FormationLeader|GetFormation%20Points) _array_index) Former%20Element)
          (Variables|BP_GoapAgent_C|SetFormation%20Position%20ID Former%20Element _array_index)
          (goto _label Break))))))

(fn IGetFormationSlotPosition
  (Utilities|IsValid (Variables|FormationElement|GetLeader%20Ref)
    (:Is%20Valid
      (return (Math|Transform|TransformLocation (Transformation|GetActorTransform (Variables|FormationElement|GetLeader%20Ref)) (.relativeposition (Utilities|Array|Get(acopy) (Variables|BP_GoapAgent_C|GetFormation%20Points (Variables|FormationElement|GetLeader%20Ref)) (Variables|FormationElement|GetFormation%20Position%20ID))))))
    (:Is%20Not%20Valid
      (Development|PrintString "FOLLOW SLOT POSITION IN AN INDIVIDUAL ENEMY" true true "(R=1.000000,G=0.000000,B=0.011039,A=1.000000)")
      ;[1 1 1] For debug and testing
      (return "0, 0, 0"))))

(fn IGetFormationSlotIndex
  (return (Variables|FormationElement|GetFormation%20Position%20ID)))