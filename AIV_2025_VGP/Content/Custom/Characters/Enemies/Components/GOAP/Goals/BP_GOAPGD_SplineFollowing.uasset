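; GOAP goal for enemy characters that expresses the drive to follow a spline.
; When elaborating the world model, it adds an insistence entry under its name, scaled from MaxInsistence by how much of the spline remains.
; Progress comes from the closest spline input key to the executer's location divided by the point count, so importance falls along the path.
; It also prints the computed importance for debugging.
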(fn ElaborateWorldModel
  (params (Wm :type GOAP%20World%20Model%20Object%20Reference))
  (bind _spline (Variables|Spline|GetSpline))
  (bind _maxinsistence (Variables|Default|GetMaxInsistence))
  (bind _executer (Variables|Default|GetExecuter))
  (bind _spline_2 (Variables|Spline|GetSpline))
  (bind _returnvalue (Transformation|GetActorLocation _executer))
  (bind _spline_3 (Variables|/Game/Custom/Characters/Enemies/BP_SplinePath.BP_SplinePath_C|GetSpline _spline))
  (bind _spline_4 (Variables|/Game/Custom/Characters/Enemies/BP_SplinePath.BP_SplinePath_C|GetSpline _spline_2))
  (bind _returnvalue_2 (Spline|GetNumberOfSplinePoints _spline_3))
  (bind _returnvalue_3 (Class|SplineComponent|FindInputKeyClosesttoWorldLocation _spline_4 _returnvalue))
  (bind _returnvalue_4 (/ _returnvalue_3 _returnvalue_2))
  (bind _returnvalue_5 (- 1.0 _returnvalue_4))
  (bind _returnvalue_6 (* _returnvalue_5 _maxinsistence))
  (Utilities|Array|AddUnique (.insistences (Variables|/Script/AIV_2025_VGP.GOAPWorldModel|GetModel Wm)) (Utilities|Struct|MakeGOAPGoal (Variables|Default|GetName) _returnvalue_6))
  (Development|PrintString 0 (Utilities|String|Append (Utilities|String|ToString(Name) (Variables|Default|GetName)) " Importance: " (Utilities|String|ToString(Float) _returnvalue_6)))
  (return Wm))