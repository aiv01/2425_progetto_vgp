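; GOAP goal component for enemy AI that sets how insistent the goal of reaching a named target position is.
; ElaborateWorldModel looks up that position in the world model and maps the executer's squared distance, clamped between desired and maximum distance, to an insistence score.
; NearIsLessImportant chooses whether insistence rises or falls with distance.
; The score is written to the model's insistences under the goal's name and debug-printed.
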(fn ElaborateWorldModel
  (params (Wm :type GOAP%20World%20Model%20Object%20Reference))
  (bind _model (Variables|/Script/AIV_2025_VGP.GOAPWorldModel|GetModel Wm))
  (bind _executer (Variables|Default|GetExecuter))
  (bind _maxinsistence (Variables|Default|GetMaxInsistence))
  (bind _target_position_name (Variables|Distances|GetTarget%20Position%20Name))
  (bind _desireddistance (Variables|Distances|GetDesiredDistance))
  (bind _maxdistance (Variables|Distances|GetMaxDistance))
  (bind _nearislessimportant_ (Variables|Distances|GetNearIsLessImportant?))
  (bind _value (Utilities|Map|Find (.positionsmodel _model) _target_position_name))
  (bind _returnvalue (Transformation|GetActorLocation _executer))
  (bind _returnvalue_2 (Math|Float|Square _maxdistance))
  (bind _returnvalue_3 (Math|Float|Square _desireddistance))
  (bind _returnvalue_4 (Class|KismetMathLibrary|VectorDistanceSquared _value _returnvalue))
  (bind _returnvalue_5 (Math|Float|MapRangeClamped _returnvalue_4 _returnvalue_3 _returnvalue_2 0.0 _maxinsistence))
  (bind _returnvalue_6 (- _maxinsistence _returnvalue_5))
  (bind _returnvalue_7 (Math|Float|SelectFloat _returnvalue_5 _returnvalue_6 _nearislessimportant_))
  ;[1 1 1] Writing insistence in the world model
  (Utilities|Array|Add (.insistences (Variables|/Script/AIV_2025_VGP.GOAPWorldModel|GetModel Wm)) (Utilities|Struct|MakeGOAPGoal (Variables|Default|GetName) _returnvalue_7))
  (Development|PrintString 0 (Utilities|String|Append (Utilities|String|ToString(Name) (Variables|Default|GetName)) " Importance" ": " (Utilities|String|ToString(Float) _returnvalue_7)))
  (return Wm))