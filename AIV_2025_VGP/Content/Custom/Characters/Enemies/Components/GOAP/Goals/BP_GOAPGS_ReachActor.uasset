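; GOAP goal that scores how strongly an enemy wants to reach a target actor, based on its distance to that actor.
; ElaborateWorldModel remaps the squared Executer-to-Target distance between desired and maximum range into an insistence capped at MaxInsistence, avoiding square roots.
; NearIsLessImportant selects whether insistence rises or falls with distance.
; The value is added to the world model under the goal's name and printed for debugging.
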(fn ElaborateWorldModel
  (params (Wm :type GOAP%20World%20Model%20Object%20Reference))
  (bind _executer (Variables|Default|GetExecuter))
  (bind _maxinsistence (Variables|Default|GetMaxInsistence))
  (bind _target (Variables|Target|GetTarget))
  (bind _desireddistance (Variables|Distances|GetDesiredDistance))
  (bind _maxdistance (Variables|Distances|GetMaxDistance))
  (bind _nearislessimportant_ (Variables|Distances|GetNearIsLessImportant?))
  (bind _returnvalue (Transformation|GetActorLocation _executer))
  (bind _returnvalue_2 (Math|Float|Square _maxdistance))
  (bind _returnvalue_3 (Math|Float|Square _desireddistance))
  (bind _returnvalue_4 (Transformation|GetActorLocation _target))
  (bind _returnvalue_5 (Class|KismetMathLibrary|VectorDistanceSquared _returnvalue_4 _returnvalue))
  (bind _returnvalue_6 (Math|Float|MapRangeClamped _returnvalue_5 _returnvalue_3 _returnvalue_2 0.0 _maxinsistence))
  (bind _returnvalue_7 (- _maxinsistence _returnvalue_6))
  (bind _returnvalue_8 (Math|Float|SelectFloat _returnvalue_6 _returnvalue_7 _nearislessimportant_))
  ;[1 1 1] Writing insistence in the world model
  (Utilities|Array|Add (.insistences (Variables|/Script/AIV_2025_VGP.GOAPWorldModel|GetModel Wm)) (Utilities|Struct|MakeGOAPGoal (Variables|Default|GetName) _returnvalue_8))
  (Development|PrintString 0 (Utilities|String|Append (Utilities|String|ToString(Name) (Variables|Default|GetName)) " Importance" ": " (Utilities|String|ToString(Float) _returnvalue_8)))
  (return Wm))