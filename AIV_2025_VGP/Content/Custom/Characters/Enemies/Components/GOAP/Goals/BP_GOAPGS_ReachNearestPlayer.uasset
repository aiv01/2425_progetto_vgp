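; GOAP goal Blueprint that rates how important reaching the nearest player is for an enemy.
; ElaborateWorldModel gets that player through an interface message on the Executer and maps their squared distance, between squared desired and max distances, to a clamped insistence.
; NearIsLessImportant selects whether insistence rises or falls with distance.
; The result is written to the world model's Insistences under the goal's Name and printed for debugging.
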(fn ElaborateWorldModel
  (params (Wm :type GOAP%20World%20Model%20Object%20Reference))
  (bind _maxinsistence (Variables|Default|GetMaxInsistence))
  (bind _nearest_player (Class|IGOAPAgent|IFindNearestPlayer(Message) (Variables|Default|GetExecuter)))
  ;[1 1 1] Writing insistence in the world model
  (Utilities|Array|Add (.insistences (Variables|/Script/AIV_2025_VGP.GOAPWorldModel|GetModel Wm)) (Utilities|Struct|MakeGOAPGoal (Variables|Default|GetName) (Math|Float|SelectFloat (Math|Float|MapRangeClamped (Class|KismetMathLibrary|VectorDistanceSquared (Transformation|GetActorLocation _nearest_player) (Transformation|GetActorLocation (Variables|Default|GetExecuter))) (Math|Float|Square (Variables|Distances|GetDesiredDistance)) (Math|Float|Square (Variables|Distances|GetMaxDistance)) 0.0 _maxinsistence) (- _maxinsistence (Math|Float|MapRangeClamped (Class|KismetMathLibrary|VectorDistanceSquared (Transformation|GetActorLocation _nearest_player) (Transformation|GetActorLocation (Variables|Default|GetExecuter))) (Math|Float|Square (Variables|Distances|GetDesiredDistance)) (Math|Float|Square (Variables|Distances|GetMaxDistance)) 0.0 _maxinsistence)) (Variables|Distances|GetNearIsLessImportant?))))
  (Development|PrintString 0 (Utilities|String|Append (Utilities|String|ToString(Name) (Variables|Default|GetName)) " Importance" ": " (Utilities|String|ToString(Float) (Math|Float|SelectFloat (Math|Float|MapRangeClamped (Class|KismetMathLibrary|VectorDistanceSquared (Transformation|GetActorLocation _nearest_player) (Transformation|GetActorLocation (Variables|Default|GetExecuter))) (Math|Float|Square (Variables|Distances|GetDesiredDistance)) (Math|Float|Square (Variables|Distances|GetMaxDistance)) 0.0 _maxinsistence) (- _maxinsistence (Math|Float|MapRangeClamped (Class|KismetMathLibrary|VectorDistanceSquared (Transformation|GetActorLocation _nearest_player) (Transformation|GetActorLocation (Variables|Default|GetExecuter))) (Math|Float|Square (Variables|Distances|GetDesiredDistance)) (Math|Float|Square (Variables|Distances|GetMaxDistance)) 0.0 _maxinsistence)) (Variables|Distances|GetNearIsLessImportant?)))))
  (return Wm))