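; BP_GOAPA_MeleeAttack is an enemy GOAP action for a melee attack.
; EvaluateFeasibility passes when the squared distance between executer and target lies within the squared minimum and maximum attack distances, avoiding a square root.
; ExecAction sends the "Jump" skill message to the executer through IExecuteSkillMessage, leaving the skill itself to be handled there.
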(event EventExecAction
  (Class|ICombatAgent|IExecuteSkill(Message) (Variables|Default|GetExecuter) "Jump"))

(fn EvaluateFeasibility
  (params (Wm :type GOAP%20World%20Model%20Object%20Reference))
  (return (Math|Float|InRange(Float) (Class|KismetMathLibrary|VectorDistanceSquared (Transformation|GetActorLocation (Variables|Attack|GetTarget%20Actor)) (Transformation|GetActorLocation (Variables|Default|GetExecuter))) (Math|Float|Square (Variables|Attack|GetAttackMinDistance)) (Math|Float|Square (Variables|Attack|GetAttackMaxDistance)))))