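; GOAP action for enemies that moves the executing character toward a named target position.
; ElaborateWorldModel looks up that position in the world model and appends a goal insistence scaled by squared distance between the desired and maximum range.
; NearIsBetter makes insistence grow with distance; otherwise it is inverted.
; ExecAction runs AI MoveTo to the cached location, using the desired distance as acceptance radius.
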(event EventExecAction
  (Development|PrintString 0 (Utilities|String|Append "GOAL: " (Utilities|String|ToString(Name) (Variables|Targt|GetInsistences%20Goal%20Name))) true true "(R=0.117799,G=1.000000,B=0.000000,A=1.000000)")
  (AI|AIMoveTo (AI|GetAIController (Variables|Default|GetExecuter)) (Variables|Targt|GetTarget%20Location) 0 (Variables|Dist|GetDesiredDistance) "Default" "Default" true true))

(fn ElaborateWorldModel
  (params (Wm :type GOAP%20World%20Model%20Object%20Reference))
  (bind _model (Variables|/Script/AIV_2025_VGP.GOAPWorldModel|GetModel Wm))
  (bind _executer (Variables|Default|GetExecuter))
  (bind _maxinsistence (Variables|Default|GetMaxInsistence))
  (bind _target_position_name (Variables|Targt|GetTarget%20Position%20Name))
  (bind _desireddistance (Variables|Dist|GetDesiredDistance))
  (bind _maxdistance (Variables|Dist|GetMaxDistance))
  (bind _insistences_goal_name (Variables|Targt|GetInsistences%20Goal%20Name))
  (bind _nearisbetter_ (Variables|Dist|GetNearIsBetter?))
  (bind _value (Utilities|Map|Find (.positionsmodel _model) _target_position_name))
  (bind _returnvalue (Transformation|GetActorLocation _executer))
  (bind _returnvalue_2 (Math|Float|Square _maxdistance))
  (bind _returnvalue_3 (Math|Float|Square _desireddistance))
  (bind _returnvalue_4 (Class|KismetMathLibrary|VectorDistanceSquared _value _returnvalue))
  (bind _returnvalue_5 (Math|Float|MapRangeClamped _returnvalue_4 _returnvalue_3 _returnvalue_2 0.0 _maxinsistence))
  (bind _returnvalue_6 (- _maxinsistence _returnvalue_5))
  (bind _returnvalue_7 (Math|Float|SelectFloat _returnvalue_5 _returnvalue_6 _nearisbetter_))
  ;[1 1 1] Find location of interest in the model
  (Variables|Targt|SetTarget%20Location _value)
  ;[1 1 1] Writing insistence in the world model
  ;;[1 0.7223 0] Problem on the not-unicity of the records inside the Model Insistence Array?
  ;;
  ;; Could it make possible error-prone situations?
  (Utilities|Array|Add (.insistences (Variables|/Script/AIV_2025_VGP.GOAPWorldModel|GetModel Wm)) (Utilities|Struct|MakeGOAPGoal _insistences_goal_name _returnvalue_7))
  (Development|PrintString 0 (Utilities|String|Append (Utilities|String|ToString(Name) _insistences_goal_name) " Importance" ": " (Utilities|String|ToString(Float) _returnvalue_7)))
  (return Wm))