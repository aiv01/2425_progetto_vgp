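; GOAP action Blueprint for enemy characters that attacks when the nearest player is within a set distance band.
; EvaluateFeasibility gets that player through an interface message on the Executer and compares squared distance against the squared min and max attack distances, avoiding a square root.
; ExecAction sends the Executer a skill message with the hardcoded name "Jump", without passing the player as a target.
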(event EventExecAction
  (Class|ICombatAgent|IExecuteSkill(Message) (Variables|Default|GetExecuter) "Jump"))

(fn EvaluateFeasibility
  (params (Wm :type GOAP%20World%20Model%20Object%20Reference))
  (bind _nearest_player (Class|IGOAPAgent|IFindNearestPlayer(Message) (Variables|Default|GetExecuter)))
  (return (Math|Float|InRange(Float) (Class|KismetMathLibrary|VectorDistanceSquared (Transformation|GetActorLocation _nearest_player) (Transformation|GetActorLocation (Variables|Default|GetExecuter))) (Math|Float|Square (Variables|Attack|GetAttackMinDistance)) (Math|Float|Square (Variables|Attack|GetAttackMaxDistance)))))