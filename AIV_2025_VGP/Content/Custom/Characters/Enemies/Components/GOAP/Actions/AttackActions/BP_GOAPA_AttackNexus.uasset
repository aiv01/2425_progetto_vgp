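; GOAP action that lets an enemy attack the Nexus by sending its executer the "Jump" skill message.
; Feasibility gets the Nexus through an interface message and checks that its distance from the executer lies between the minimum and maximum attack distances.
; The check compares squared distances, optionally adding the executer's scaled capsule radius to the distance before squaring.
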(event EventExecAction
  (Class|ICombatAgent|IExecuteSkill(Message) (Variables|Default|GetExecuter) "Jump"))

(fn EvaluateFeasibility
  (params (Wm :type GOAP%20World%20Model%20Object%20Reference))
  (bind _executer (Variables|Default|GetExecuter))
  (bind _returnvalue (Transformation|GetActorLocation _executer))
  (bind _nexus (Class|IGOAPAgent|IGetNexus(Message) (Variables|Default|GetExecuter)))
  ;[1 1 1] "Is in Melee Range?" Logic
  (return (Math|Float|InRange(Float) (Math|Float|SelectFloat (Math|Float|Square (+ (Components|Capsule|GetScaledCapsuleRadius (Variables|/Script/Engine.Character|GetCapsuleComponent (Variables|Default|GetExecuter))) (Math|Vector|Distance(Vector) (Transformation|GetActorLocation (Utilities|Array|Get(acopy) _nexus)) _returnvalue))) (Class|KismetMathLibrary|VectorDistanceSquared (Transformation|GetActorLocation (Utilities|Array|Get(acopy) _nexus)) _returnvalue) (Variables|Distances|GetConsider%20Capsule%20Radius?)) (Math|Float|Square (Variables|Distances|GetAttackMinDistance)) (Math|Float|Square (Variables|Distances|GetAttackMaxDistance)))))