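; GOAP movement action that moves its executing pawn along a spline.
; On initialization it gets the spline from the executer through an interface message and caches it.
; On execution it finds the input key closest to the pawn, adds a forwarding offset clamped to the spline's point count, and issues AI MoveTo toward that world location.
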(event EventExecAction
  (bind _spline (Variables|SplineFollow|GetSpline))
  (bind _executer (Variables|Default|GetExecuter))
  (bind _spline_2 (Variables|/Game/Custom/Characters/Enemies/BP_SplinePath.BP_SplinePath_C|GetSpline _spline))
  (AI|AIMoveTo _executer _executer (Class|SplineComponent|GetLocationatSplineInputKey _spline_2 (Math|Float|Clamp(Float) (+ (Class|SplineComponent|FindInputKeyClosesttoWorldLocation _spline_2 (Transformation|GetActorLocation (Variables|Default|GetExecuter))) (Variables|SplineFollow|GetForwarding)) 0.0 (Math|Conversions|ToFloat(Integer) (Spline|GetNumberOfSplinePoints _spline_2))) "World") 0 5.0 false))

(event EventInitializeAction
  (bind _spline_path (Class|IGOAPAgent|IGetSplinetoFollow(Message) (Variables|Default|GetExecuter)))
  (Variables|SplineFollow|SetSpline _spline_path))