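; GOAP agent component that drives enemy decision-making through goals and actions bound to the owning BaseEnemy at BeginPlay.
; ChoseGoal schedules Planning on a short randomized timer.
; Once the minimum execution time has elapsed, Planning has goals elaborate the world model to set insistences, then runs a depth-limited plan and executes the resulting action.
; Until then, it re-executes the current action.
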(event Custom|Chose%20Goal
  (params (wdModel :type GOAP%20World%20Model%20Object%20Reference))
  (bind _returnvalue (Utilities|Time|SetTimerbyEvent (delegate Custom|Planning) (Math|Random|RandomFloatinRange 0.0 0.6)))
  (Variables|Planning|SetPlanning%20Timer _returnvalue))

(event Custom|Planning
  (if (>= (- (Utilities|Time|GetTimeSeconds) (Variables|ActionsTiming|GetLast%20Action%20Time)) (Variables|ActionsTiming|GetMin%20Action%20Execution%20Time))
    (Utilities|IsValid (stale Custom|Chose%20Goal wdModel)
      (:Is%20Valid
        (CallFunction|ElaborateWorldModel (stale Custom|Chose%20Goal wdModel))
        ;[1 1 1] GOAP
        (bind _returnvalue (Class|GOAPAgentComponent|PlanAction (stale Custom|Chose%20Goal wdModel) (Variables|Planning|GetPlanning%20Depth)))
        (Utilities|IsValid _returnvalue
          (:Is%20Valid
            (Development|PrintString (Utilities|String|Append "BEST ACTION IS: " (Utilities|GetDisplayName _returnvalue)) true true "(R=0.052031,G=1.000000,B=0.000000,A=1.000000)")
            (Variables|Default|SetCurrent%20Action _returnvalue)
            (Class|GOAPAction|ExecAction _returnvalue)
            (Variables|ActionsTiming|SetLast%20Action%20Time (Utilities|Time|GetTimeSeconds))))))
    (else
      (Class|GOAPAction|ExecAction (Variables|Default|GetCurrent%20Action)))))

(event EventBeginPlay
  (Development|PrintString "GOAP Component activated" true true "(R=1.000000,G=0.792499,B=0.000000,A=1.000000)")
  (Utilities|FlowControl|Sequence
    (:then_0
      (for _array_element (Variables|Default|GetActions)
        (bind _asbase_enemy (Utilities|Casting|CastToBaseEnemy (Components|GetOwner)))
        (Variables|/Script/AIV_2025_VGP.GOAPAction|SetExecuter _array_element _asbase_enemy)
        (Class|GOAPAction|InitializeAction _array_element)))
    (:then_1
      (for _array_element_2 (Variables|Default|GetGoals)
        (bind _asbase_enemy_2 (Utilities|Casting|CastToBaseEnemy (Components|GetOwner)))
        (Variables|/Script/AIV_2025_VGP.GOAPGoalDefiner|SetExecuter _array_element_2 _asbase_enemy_2)))))

(fn ElaborateWorldModel
  (params (WorldMd :type GOAP%20World%20Model%20Object%20Reference))
  (for _array_element (Variables|Default|GetGoals)
    ;[1 1 1] Elaborate World Model to define insistences
    (Class|GOAPGoalDefiner|ElaborateWorldModel _array_element WorldMd)))