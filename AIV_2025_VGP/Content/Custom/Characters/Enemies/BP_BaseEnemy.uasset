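; BP_BaseEnemy is the base enemy character, exposing movement and skill interfaces.
; Its moving-agent functions report current speed, rescale velocity to a new speed along its current direction, and return the SplinePath to follow.
; A separate UpdateWalkSpeed function sets the CharacterMovement max walk speed.
; Skill execute and end events are empty here, as are BeginPlay and the construction script.
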(event EventBeginPlay)

(event EventIEndSkill
  (params (SkillName :type Name :default "None")))

(event EventIExecuteSkill
  (params (SkillName :type Name :default "None")))

(event EventISetSpeed
  (params (NewSpeed :type Float%20%28single-precision%29))
  (bind _charactermovement (Variables|Character|GetCharacterMovement))
  (Variables|/Script/Engine.MovementComponent|SetVelocity _charactermovement (* NewSpeed (Math|Vector|Normalize (Variables|/Script/Engine.MovementComponent|GetVelocity _charactermovement)))))

(fn ConstructionScript)

(fn UpdateWalkSpeed
  (params (WalkSpeed :type Float%20%28double-precision%29))
  (Variables|/Script/Engine.CharacterMovementComponent|SetMaxWalkSpeed (Variables|Character|GetCharacterMovement) WalkSpeed))

(fn IGetSpeed
  (return (Math|Vector|VectorLength (Variables|/Script/Engine.MovementComponent|GetVelocity (Variables|Character|GetCharacterMovement)))))

(fn IGetSplinetoFollow
  (return (Variables|Movement|GetSpline%20Path)))