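; BP_SplinePath is a spline path actor in the enemy character folder that records its point positions, likely for enemy movement.
; On BeginPlay it counts and logs the spline points, then caches each position in the SplinePointsPosition array.
; Each cached value adds the spline component's world location to the point's already world-space position.
; A temporary red debug sphere marks each computed position.
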(event EventBeginPlay
  (bind _spline (Variables|Default|GetSpline))
  ;[1 1 1] Calculate spline points count
  (bind _output_get (Variables|Default|SetSplinePointsCount (Spline|GetNumberOfSplinePoints (Variables|Default|GetSpline))))
  (Utilities|String|LogString (Utilities|String|Append "SplinePoints found: " (Utilities|String|ToString(Integer) _output_get)))
  ;[1 1 1] Calculate world position of each spline points
  (for _index (range 0 (- (Variables|Default|GetSplinePointsCount) 1))
    (Rendering|Debug|DrawDebugSphere (+ (Transformation|GetWorldLocation _spline) (.position (Spline|GetSplinePointAt _spline _index "World"))) 2e+01 12 "(R=1.000000,G=0.000000,B=0.018015,A=1.000000)" 2e+01 1.0)
    (Utilities|Array|Add (Variables|Default|GetSplinePointsPosition) (+ (Transformation|GetWorldLocation _spline) (.position (Spline|GetSplinePointAt _spline _index "World"))))))

(fn ConstructionScript)