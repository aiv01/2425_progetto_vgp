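; BP_AIManager maintains the shared GOAP world model for enemy AI and initializes enemies spawned by the wave manager.
; On BeginPlay it creates the model, loading static data from a Level1 DataTable row and adding condition keys.
; A looping timer clears insistences, records player pawn positions and broadcasts the model.
; Each spawned GOAP agent is bound to those updates, given the spline path and Nexus, then initialized.
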(event Custom|World%20State%20Update
  (CallFunction|CalculateWorldState)
  (Default|CallNotifyWorldUpdate (Variables|WorldModel|GetCurrent%20World%20Model)))

(event Custom|Initialize%20Enemies
  (params (EnemySpawn :type Actor%20Object%20Reference))
  (CallFunction|EnemyInitialization EnemySpawn))

(event Custom|Stop%20World%20State%20Update
  (Utilities|Time|ClearandInvalidateTimerbyHandle (Variables|WorldModel|GetWorld%20State%20Update%20Timer)))

(event EventBeginPlay
  (bind _returnvalue (Game|ConstructObjectfromClass "/Script/AIV_2025_VGP.GOAPWorldModel"))
  (Variables|WorldModel|SetCurrent%20World%20Model _returnvalue)
  (EventDispatchers|BindEventtoOnEnemySpawn (Variables|Default|GetWaveMNG) (delegate Custom|Initialize%20Enemies))
  (CallFunction|InsertKeystoWorldState)
  (bind _returnvalue_2 (Utilities|Time|SetTimerbyEvent (delegate Custom|World%20State%20Update) (Variables|WorldModel|GetAI%20Update%20Time) true))
  (Variables|WorldModel|SetWorld%20State%20Update%20Timer _returnvalue_2))

(fn ConstructionScript)

(fn CalculateWorldState
  ;[1 1 1] Cleaning of the previous informations
  (Utilities|Array|Clear (.insistences (Variables|/Script/AIV_2025_VGP.GOAPWorldModel|GetModel (Variables|WorldModel|GetCurrent%20World%20Model))))
  (for _index (range 0 (- (Class|GameplayStatics|GetNumPlayerControllers) 1))
    (Utilities|Map|Add (.positionsmodel (Variables|/Script/AIV_2025_VGP.GOAPWorldModel|GetModel (Variables|WorldModel|GetCurrent%20World%20Model))) (Utilities|String|StringToName (Utilities|String|Append "Player" (Utilities|String|ToString(Integer) _index))) (Transformation|GetActorLocation (Game|Player|GetPlayerPawn _index))))
  (return))

(fn InsertKeystoWorldState
  (Utilities|FlowControl|Sequence
    (:then_0
      ;[1 1 1] Static Model Variables, loaded by a Data Table basing on the level
      (bind _returnvalue (Utilities|GetDataTableRow "/Game/Custom/Characters/Enemies/Components/GOAP/DT_WorldModels.DT_WorldModels" "Level1")
        (:then
          (Variables|/Script/AIV_2025_VGP.GOAPWorldModel|SetModel (Variables|WorldModel|GetCurrent%20World%20Model) _returnvalue))))
    (:then_1
      (Utilities|Map|Add (.conditionsmodel (Variables|/Script/AIV_2025_VGP.GOAPWorldModel|GetModel (Variables|WorldModel|GetCurrent%20World%20Model))) "Player0Alive" true)
      (Utilities|Map|Add (.conditionsmodel (Variables|/Script/AIV_2025_VGP.GOAPWorldModel|GetModel (Variables|WorldModel|GetCurrent%20World%20Model))) "Plipli" false))))

(fn EnemyInitialization
  (params (Object :type Object%20Object%20Reference))
  (bind _asbp_goap_agent (Utilities|Casting|CastToBP_GoapAgent Object))
  (LocalVariables|SetEnemy _asbp_goap_agent)
  (Utilities|FlowControl|Sequence
    (:then_0
      (Class|AIManager|BindtoWorldUpdate (LocalVariables|GetEnemy))
      (Variables|/Game/Custom/Characters/Enemies/BP_BaseEnemy.BP_BaseEnemy_C|SetSpline%20Path (LocalVariables|GetEnemy) (Variables|World'sInstances|GetSpline%20Path))
      (Utilities|Array|AddUnique (Variables|/Game/Custom/Characters/Enemies/ConcreteEnemies/BP_GoapAgent.BP_GoapAgent_C|GetNexus (LocalVariables|GetEnemy)) (Variables|Default|GetNexus)))
    (:then_1
      (Default|InitAI (LocalVariables|GetEnemy))
      (Default|InitGOAP (LocalVariables|GetEnemy)))))