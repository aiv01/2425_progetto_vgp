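; Multiplayer co-op player character with HUD, weapon switching, ability-based attacks and friend revival.
; Health component events update the HUD and drive the knocked state, which disables input and enlarges a sphere so nearby players can revive.
; Teammates register one at a time, chained on Steam avatar callbacks, to fill team health bars.
; Primary attack replicates via server-to-multicast RPC, secondary executes directly; debug keys and a death stub remain.
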(event OnComponentBeginOverlap(Sphere)
  (params (OverlappedComponent :type Primitive%20Component%20Object%20Reference) (OtherActor :type Actor%20Object%20Reference) (OtherComp :type Primitive%20Component%20Object%20Reference) (OtherBodyIndex :type Integer) (bFromSweep :type Boolean) (SweepResult :type Hit%20Result%20Structure%20%28by%20ref%29))
  ;[0 1 0.915] Revive System
  ;;[1 1 1 0.5] RPC Collider
  (if (CallFunction|Revive-IsPlayer OtherActor)
    (if (Variables|Health|GetIsLanded)
      (Class|HealthComponent|ChangeReviveFriendStatus (Variables|Default|GetHealth) OtherActor true self))))

(event OnComponentEndOverlap(Sphere)
  (params (OverlappedComponent :type Primitive%20Component%20Object%20Reference) (OtherActor :type Actor%20Object%20Reference) (OtherComp :type Primitive%20Component%20Object%20Reference) (OtherBodyIndex :type Integer))
  ;[0 1 0.915] Revive System
  ;;[1 1 1 0.5] RPC Collider
  (if (CallFunction|Revive-IsPlayer OtherActor)
    (if (Variables|Health|GetIsLanded)
      (Class|HealthComponent|ChangeReviveFriendStatus (Variables|Default|GetHealth) OtherActor false))))

(event Custom|IsKnockedEvent
  ;[0 1 0] Health System
  ;;[1 1 1 0.5] Landed Event
  (Development|PrintString "Landed")
  (CallFunction|DisableContextMap)
  (Variables|Health|SetIsLanded true)
  (Components|Sphere|SetSphereRadius (Variables|Default|GetSphere) 1e+02 true))

(event Custom|IsDeadEvent
  ;[0 1 0] Health System
  ;;[1 1 1 0.5] Death Event // TO DO
  (Development|PrintString "Death"))

(event Custom|OnGetAvatar
  (params (RequestedFriendAvatar :type Texture%202D%20Object%20Reference))
  ;[1 0.1156 0] UI Friend List
  ;;[1 1 1] Client RPC
  (CallFunction|UpdateHUD-AddNewFriend RequestedFriendAvatar)
  (CallFunction|Util-BindChangeHealth)
  (CallFunction|UpdateOtherClient (Variables|HUD|Friendlist|GetCurrent%20Target) self)
  (if (CallFunction|Util-OutOfIndex)
    (Variables|HUD|Friendlist|SetLoopIndex -1)
    (elif (not (CallFunction|Util-CicleEnd))
      (bind _result (Math|Integer|IncrementInt (Variables|HUD|Friendlist|GetLoopIndex))
        (:%20%20
          (CallFunction|Util-CustomLoop _result))))))

(event Custom|Multicast_ReplicatesMoveLocalPlayer
  (params (NewLocation :type Vector))
  ;[1 1 1] Move all Players
  (bind _asbase_player_controller (Utilities|Casting|CastToBasePlayerController (Pawn|GetController)))
  (for _array_element (Class|BasePlayerController|GetAllBasePlayers _asbase_player_controller)
    (Utilities|IsValid _array_element
      (:Is%20Valid
        (Transformation|SetActorLocation _array_element NewLocation false false)))))

(event Custom|UpdateImage
  (params (CSteamID :type Integer))
  ;[1 0.1156 0] UI Friend List
  ;;[1 1 1 0.5] Server RPC
  (Variables|HUD|Friendlist|SetCSteamID CSteamID))

(event Custom|ServerRPC_ExecuteCommand
  (params (Caller :type BP%20Main%20Character%20Object%20Reference) (InputPin :type Name))
  (CallFunction|MulticastRPCExecuteCommand Caller InputPin))

(event Custom|ChangeOtherHealth
  (params (Instigator :type Actor%20Object%20Reference))
  ;[0 1 0] Health System
  ;;[1 1 1 0.5] Update For All Friend
  (bind (_array_element _array_index) (Utilities|Array|ForEachLoopwithBreak (Variables|HUD|Friendlist|GetOut%20Actors) :!label _label)
    (:LoopBody
      (if (== _array_element Instigator)
        (bind _asbp_main_character (Utilities|Casting|CastToBP_MainCharacter _array_element))
        (CallFunction|UpdateHUD-Friends _asbp_main_character _array_index)
        (goto _label Break)))))

(event Custom|ChangeHealth
  (params (Actor :type Actor%20Object%20Reference))
  ;[0 1 0] Health System
  ;;[1 1 1 0.5] Change Health Callback
  (CallFunction|UpdateHUD-Health)
  (if (CallFunction|Revive-ChangeReviveStatus)
    (Components|Sphere|SetSphereRadius (Variables|Default|GetSphere) 0.0 true)
    (CallFunction|EnableContextMap)
    (Variables|Health|SetIsLanded false)
    (Class|HealthComponent|StopLandedTimer (Variables|Default|GetHealth))))

(event Custom|ClientUpdate
  ;[1 0.1156 0] UI Friend List
  ;;[1 1 1] Client RPC
  (bind _asbase_player_controller (Utilities|Casting|CastToBasePlayerController (Pawn|GetController)))
  (Variables|HUD|Friendlist|SetTempPlayers (Class|BasePlayerController|GetAllBasePlayers _asbase_player_controller))
  (bind _output_get (Variables|HUD|Friendlist|SetLoopIndex 0))
  (CallFunction|Util-CustomLoop _output_get))

(event Custom|UpdateOtherClient
  (params (Target :type Actor%20Object%20Reference) (NewActor :type Actor%20Object%20Reference))
  ;[1 0.1156 0] UI Friend List
  ;;[1 1 1 0.5] Server RPC
  (Class|BPIMultiplayerInterfaces|IUpdateFriends(Message) Target NewActor))

(event Custom|AddNewPlayer
  (params (NewItem :type Actor%20Object%20Reference%20%28by%20ref%29))
  ;[1 0.1156 0] UI Friend List
  ;;[1 1 1] Client RPC
  (CallFunction|HUD-AddNewPlayer NewItem)
  (Variables|HUD|Friendlist|SetLoopIndex -1))

(event Custom|MulticastRPC_ExecuteCommand
  (params (Target :type BP%20Main%20Character%20Object%20Reference) (InputPin :type Name))
  ;[0 0.1538 1] Weapon
  ;;[1 1 1 0.5] Attack Inputs
  (Class|AbilitySystemComponent|ExecuteStrategy (Variables|BP_MainCharacter_C|GetAbilitySystem Target) InputPin))

(event EventChangeWeapon
  (params (bForward :type Boolean))
  ;[0 0.1538 1] Weapon
  ;;[1 1 1 0.5] Change Weapon Input
  (Class|BaseWeaponComponent|ChangeWeapon (Variables|Default|GetBPC_BaseWeapon) bForward)
  (CallFunction|UpdateHUD-Weapon))

(event EventBeginPlay
  ;[0.7632 0 1] BeginPlay
  (bind _asbase_player_controller (Utilities|Casting|CastToBasePlayerController (Pawn|GetController)))
  (bind _returnvalue (UserInterface|CreateWidget "/Game/Custom/Networking/Widgets/WBP_PauseMenu.WBP_PauseMenu_C" _asbase_player_controller))
  (Variables|Default|SetPauseMenu _returnvalue)
  (CallFunction|HUD-CreateHUD _asbase_player_controller)
  (CallFunction|Health-BindEvents)
  (bind _returnvalue_2 (Class|PNetworkingInstanceSteam|GetUniqueInstance))
  (bind (_outsteamid _returnvalue_3) (Class|PNetworkingInstanceSteam|GetLocalCSteamID _returnvalue_2))
  (if _returnvalue_3
    (CallFunction|UpdateImage _outsteamid)))

(event EventPrimaryAttack
  (CallFunction|ServerRPCExecuteCommand self (Class|BaseWeaponComponent|GetPrimaryAttackName (Variables|Default|GetBPC_BaseWeapon))))

(event EventSecondaryAttack
  ;[0 0.1538 1] Weapon
  ;;[1 1 1 0.5] Attack Inputs
  (Class|AbilitySystemComponent|ExecuteStrategy (Variables|Default|GetAbilitySystem) (Class|BaseWeaponComponent|GetSecondaryAttackName (Variables|Default|GetBPC_BaseWeapon))))

(event EventISetHealth
  (params (Delta :type Float%20%28single-precision%29))
  ;[0 1 0] Health System
  ;;[1 1 1 0.5] Health Interface
  (Class|HealthComponent|ChangeHealth (Variables|Default|GetHealth) Delta))

(event EventIPostLogin
  ;[1 0.1156 0] UI Friend List
  ;;[1 1 1 0.5] Update Interfaces
  (CallFunction|ClientUpdate))

(event EventIFriendCanRevive
  (params (bNewStatus :type Boolean) (SelfRef :type Actor%20Object%20Reference))
  ;[0 1 0.915] Revive System
  ;;[1 1 1 0.5] Revive Interface
  (Variables|Health|Revive|SetFriendToRev bNewStatus)
  (Variables|Health|Revive|SetActorToRevive SelfRef))

(event EventRevive
  ;[0 1 0.915] Revive System
  ;;[1 1 1 0.5] Input For Revive
  (if (Variables|Health|Revive|GetFriendToRev)
    (bind _actortorevive (Variables|Health|Revive|GetActorToRevive)
      (:then
        (Class|HealthComponent|HealtoActor (Variables|Default|GetHealth) 1e+01 _actortorevive self)
        (Class|HealthComponent|StopLandedTimer (Variables|Default|GetHealth)))
      (:else))))

(event EventIUpdateFriends
  (params (NewActor :type Actor%20Object%20Reference))
  ;[1 0.1156 0] UI Friend List
  ;;[1 1 1 0.5] Update Interfaces
  (CallFunction|AddNewPlayer NewActor))

(event EventIMoveLocalPlayer
  (params (NewPos :type Vector :default "0, 0, 0"))
  ;[1 1 1] Move all Players
  (Networking|SwitchHasAuthority
    (:Authority
      (CallFunction|MulticastReplicatesMoveLocalPlayer NewPos))))

(event Input|KeyboardEvents|R
  (params (Key :type Key%20Structure :default "None"))
  ;[1 1 1] TO REMOVE
  (:Pressed
    (Class|BaseWeaponComponent|AddNewWeapon (Variables|Default|GetBPC_BaseWeapon) "/Game/Custom/Characters/MainCharacter/Weapons/BP_fist.BP_fist_C")))

(event Input|KeyboardEvents|P
  (params (Key :type Key%20Structure :default "None"))
  (bind _pausemenu (Variables|Default|GetPauseMenu))
  ;[1 1 1] Pause menu
  (:Pressed
    (UserInterface|Viewport|AddtoViewport _pausemenu 0)
    (Default|SetUpParty _pausemenu (Variables|HUD|Friendlist|GetOut%20Actors))))

(event Input|KeyboardEvents|Z
  (params (Key :type Key%20Structure :default "None"))
  ;[1 1 1] TEST
  (:Pressed
    (CallFunction|ISetHealth 1e+01)))

(event Input|KeyboardEvents|X
  (params (Key :type Key%20Structure :default "None"))
  ;[1 1 1] TEST
  (:Pressed
    (CallFunction|ISetHealth -1e+01)))

(event Input|KeyboardEvents|B
  (params (Key :type Key%20Structure :default "None"))
  ;[1 1 1] TEST
  (:Pressed
    (for _array_element (Variables|HUD|Friendlist|GetOut%20Actors)
      (Class|HealthComponent|HealtoActor (Variables|Default|GetHealth) 1e+01 _array_element self))))

(event Input|KeyboardEvents|V
  (params (Key :type Key%20Structure :default "None"))
  ;[1 1 1] TEST
  (:Pressed
    (for _array_element (Variables|HUD|Friendlist|GetOut%20Actors)
      (Class|HealthComponent|MakeDamagetoActor (Variables|Default|GetHealth) 1e+01 _array_element self))))

(fn ConstructionScript)

(fn UpdateHUD-Weapon
  (bind _returnvalue (Utilities|GetDataTableRow "/Game/Custom/Characters/MainCharacter/Table/DT_WeaponsImage.DT_WeaponsImage" (Variables|/Script/AIV_2025_VGP.BaseWeaponComponent|GetCurrentWeaponName (Variables|Default|GetBPC_BaseWeapon)))
    (:then
      (Class|Image|SetBrush (Variables|/Game/Custom/Characters/MainCharacter/HUD/Widgets/WBP_HUD.WBP_HUD_C|GetWeaponImage (Variables|HUD|GetHUD)) (Utilities|Struct|MakeSlateBrush "Image" "NoTile" "NoMirror" "(X=32.000000,Y=32.000000)" "(Left=0.000000,Top=0.000000,Right=0.000000,Bottom=0.000000)" "(SpecifiedColor=(R=1.000000,G=1.000000,B=1.000000,A=1.000000),ColorUseRule=UseColor_Specified)" "(CornerRadii=(X=0.000000,Y=0.000000,Z=0.000000,W=0.000000),Color=(SpecifiedColor=(R=0.000000,G=0.000000,B=0.000000,A=0.000000),ColorUseRule=UseColor_Specified),Width=0.000000,RoundingType=HalfHeightRadius,bUseBrushTransparency=False)" (.image _returnvalue))))))

(fn UpdateHUD-Friends
  (params (Target :type BP%20Main%20Character%20Object%20Reference) (Index :type Integer))
  (Default|UpdatePlayer (Variables|/Game/Custom/Characters/MainCharacter/HUD/Widgets/WBP_HUD.WBP_HUD_C|GetWBP_TeamHealth (Variables|HUD|GetHUD)) (Class|HealthComponent|GetPercentHealth (Variables|BP_MainCharacter_C|GetHealth Target)) Index))

(fn UpdateHUD-AddNewFriend
  (params (Brush%20Image :type Texture%202D%20Object%20Reference))
  (Default|AddNewPlayer (Variables|/Game/Custom/Characters/MainCharacter/HUD/Widgets/WBP_HUD.WBP_HUD_C|GetWBP_TeamHealth (Variables|HUD|GetHUD)) Brush%20Image (Variables|HUD|Friendlist|GetCurrent%20Player%20ID)))

(fn UpdateHUD-Health
  (Default|UpdateHealth (Variables|HUD|GetHUD) (Variables|/Script/HealthSystem.HealthComponent|GetHealth (Variables|Default|GetHealth))))

(fn UpdateHUD
  (CallFunction|UpdateHUD-Weapon)
  (CallFunction|UpdateHUD-Health))

(fn HUD-CreateHUD
  (params (OwningPlayer :type Player%20Controller%20Object%20Reference))
  (bind _returnvalue (UserInterface|CreateWidget "/Game/Custom/Characters/MainCharacter/HUD/Widgets/WBP_HUD.WBP_HUD_C" OwningPlayer))
  (bind _output_get (Variables|HUD|SetHUD _returnvalue))
  (UserInterface|Viewport|AddtoViewport _output_get 0)
  (CallFunction|UpdateHUD))

(fn HUD-AddNewPlayer
  (params (NewPlayer :type Actor%20Object%20Reference%20%28by%20ref%29))
  (bind _returnvalue (Utilities|Array|AddUnique (Variables|HUD|Friendlist|GetOut%20Actors) NewPlayer))
  (if (!= _returnvalue -1)
    (Variables|HUD|Friendlist|SetCurrent%20Player%20ID _returnvalue)
    (bind _output_get (Variables|HUD|Friendlist|SetCurrent%20Target NewPlayer))
    (bind _csteamid (Class|BPIMultiplayerInterfaces|IUpdateImage(Message) _output_get))
    (bind _returnvalue_2 (Class|PNetworkingInstanceSteam|GetUniqueInstance))
    (Class|PNetworkingInstanceSteam|GetAvatarfromSteamID _returnvalue_2 _csteamid (EventDispatchers|CreateEvent :!event Custom|OnGetAvatar))
    (elif (not (or (CallFunction|Util-OutOfIndex) (CallFunction|Util-CicleEnd)))
      (bind _result (Math|Integer|IncrementInt (Variables|HUD|Friendlist|GetLoopIndex))
        (:%20%20
          (CallFunction|Util-CustomLoop _result))))))

(fn IsHUDOwner
  (return (== (Widget|GetOwningPlayer (Variables|HUD|GetHUD)) (Pawn|GetController))))

(fn DisableContextMap
  (bind _asbase_player_controller (Utilities|Casting|CastToBasePlayerController (Pawn|GetController)))
  (Class|EnhancedInputSubsystemInterface|ClearAllMappings (PlayerController|LocalPlayerSubsystems|GetEnhancedInputLocalPlayerSubsystem _asbase_player_controller)))

(fn EnableContextMap
  (bind _asbase_player_controller (Utilities|Casting|CastToBasePlayerController (Pawn|GetController)))
  (Input|AddMappingContext (PlayerController|LocalPlayerSubsystems|GetEnhancedInputLocalPlayerSubsystem _asbase_player_controller) "/Game/Custom/Characters/MainCharacter/Inputs/IMC_MainCharacter.IMC_MainCharacter" 3 "(bIgnoreAllPressedKeysUntilRelease=True,bForceImmediately=False,bNotifyUserSettings=False)"))

(fn Revive-ChangeReviveStatus
  (return (and (Variables|Health|GetIsLanded) (> (Variables|/Script/HealthSystem.HealthComponent|GetHealth (Variables|Default|GetHealth)) 0.0))))

(fn Revive-IsPlayer
  (params (Actor :type Actor%20Object%20Reference))
  (return (and (Actor|ActorHasTag Actor "Player") (not (== Actor self)))))

(fn Util-NotMe
  (params (Actor :type Object%20Object%20Reference))
  (return (not (== Actor self))))

(fn Util-Me
  (params (Actor :type Object%20Object%20Reference))
  (return (== Actor self)))

(fn Util-BindChangeHealth
  (EventDispatchers|BindEventtoOnChangeHealth (Actor|GetComponentbyClass (Variables|HUD|Friendlist|GetCurrent%20Target) "/Script/HealthSystem.HealthComponent") (EventDispatchers|CreateEvent :!event Custom|ChangeOtherHealth)))

(fn Util-GetController)

(fn Util-CustomLoop
  (params (Index :type Integer))
  (bind _tempplayers (Variables|HUD|Friendlist|GetTempPlayers))
  (bind _output (Utilities|Array|Get(acopy) _tempplayers Index))
  (if (CallFunction|Util-NotMe _output)
    (CallFunction|HUD-AddNewPlayer _output)
    (elif (not (or (CallFunction|Util-OutOfIndex) (CallFunction|Util-CicleEnd)))
      (bind _result (Math|Integer|IncrementInt (Variables|HUD|Friendlist|GetLoopIndex))
        (:%20%20
          (CallFunction|Util-CustomLoop _result))))))

(fn Util-OutOfIndex
  (return (>= (Variables|HUD|Friendlist|GetLoopIndex) (- (Utilities|Array|Length (Variables|HUD|Friendlist|GetTempPlayers)) 1))))

(fn Util-CicleEnd
  (return (== (Variables|HUD|Friendlist|GetLoopIndex) -1)))

(fn Health-BindEvents
  (EventDispatchers|BindEventtoOnLanded (Variables|Default|GetHealth) (EventDispatchers|CreateEvent :!event Custom|IsKnockedEvent))
  (EventDispatchers|BindEventtoOnDeath (Variables|Default|GetHealth) (EventDispatchers|CreateEvent :!event Custom|IsDeadEvent))
  (EventDispatchers|BindEventtoOnChangeHealth (Variables|Default|GetHealth) (EventDispatchers|CreateEvent :!event Custom|ChangeHealth)))

(fn IUpdateImage
  (return (Variables|HUD|Friendlist|GetCSteamID)))