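; BP_Sword is a main-character melee weapon that uses a Box component as its hit volume.
; The box starts without collision, and the primary attack start and end events toggle it between query-only and disabled to limit hits to the attack window.
; Overlaps with actors not tagged Player only print a debug message, as damage is still a ToDo.
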(event OnComponentBeginOverlap(Box)
  (params (OverlappedComponent :type Primitive%20Component%20Object%20Reference) (OtherActor :type Actor%20Object%20Reference) (OtherComp :type Primitive%20Component%20Object%20Reference) (OtherBodyIndex :type Integer) (bFromSweep :type Boolean) (SweepResult :type Hit%20Result%20Structure%20%28by%20ref%29))
  (if (not (Actor|ActorHasTag OtherActor "Player"))
    ;[1 1 1] ToDo MakeDamage
    (Development|PrintString "MakeDamage")))

(event EventPrimaryAttackEventStart
  (Collision|SetCollisionEnabled (Variables|Default|GetBox) "QueryOnly")
  (Development|PrintString "Collisio Enable"))

(event EventBeginPlay
  (Collision|SetCollisionEnabled (Variables|Default|GetBox) "NoCollision"))

(event EventPrimaryAttackEventEnd
  (Collision|SetCollisionEnabled (Variables|Default|GetBox) "NoCollision")
  (Development|PrintString "Collisio Disable"))

(fn ConstructionScript)