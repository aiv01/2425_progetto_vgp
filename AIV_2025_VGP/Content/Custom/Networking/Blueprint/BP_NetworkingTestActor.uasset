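; Test actor that exercises online subsystem calls by printing the app ID, account name and friend lists to the screen.
; On BeginPlay it prints the app ID and local user's account name, then after a short delay requests the online friends list.
; That callback prints the names, then after a further delay requests the full friends list.
; A shared TestPrintFriendlist function prints each name if its request returned true.
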(event Custom|PrintOnlineFriendsList
  (params (FriendsListNames :type Array%20of%20Strings))
  (CallFunction|TestPrintFriendlist (stale EventBeginPlay _returnvalue_3) FriendsListNames)
  (Utilities|FlowControl|Delay 15.0)
  (bind _returnvalue (Class|PNetworkingBPLibrary|GetAllFriendsList (delegate Custom|PrintAllFriendsList))))

(event Custom|PrintAllFriendsList
  (params (FriendsListNames :type Array%20of%20Strings))
  (CallFunction|TestPrintFriendlist (stale Custom|PrintOnlineFriendsList _returnvalue) FriendsListNames))

(event EventBeginPlay
  (Utilities|FlowControl|Sequence
    (:then_0
      (bind (_appid _returnvalue) (Class|PNetworkingBPLibrary|GetAppID))
      (if _returnvalue
        (Development|PrintString _appid)))
    (:then_1
      (bind (_accountname _returnvalue_2) (Class|PNetworkingBPLibrary|GetAccountName))
      (if _returnvalue_2
        (Development|PrintString _accountname)))
    (:then_2
      (Utilities|FlowControl|Delay 5.0)
      (bind _returnvalue_3 (Class|PNetworkingBPLibrary|GetOnlineFriendsList (delegate Custom|PrintOnlineFriendsList))))))

(fn ConstructionScript)

(fn TestPrintFriendlist
  (params (Condition :type Boolean) (InputPin :type Array%20of%20Strings))
  (if Condition
    (for _array_element InputPin
      (Development|PrintString _array_element true true "(R=0.000000,G=0.660000,B=1.000000,A=1.000000)" 1e+01))))