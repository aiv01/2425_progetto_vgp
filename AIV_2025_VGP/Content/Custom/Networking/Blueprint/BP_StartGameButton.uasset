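; BP_StartGameButton is an overlap trigger that lets the host start the game from a networked session.
; When a tagged Player that is locally controlled and has authority enters the box, it disables its collision so it fires once.
; It then messages the GameInstance to close session joinability and tells that player to move to the TPTarget location through interface calls.
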(event OnComponentBeginOverlap(Box)
  (params (OverlappedComponent :type Primitive%20Component%20Object%20Reference) (OtherActor :type Actor%20Object%20Reference) (OtherComp :type Primitive%20Component%20Object%20Reference) (OtherBodyIndex :type Integer) (bFromSweep :type Boolean) (SweepResult :type Hit%20Result%20Structure%20%28by%20ref%29))
  ;[1 1 1] Overlap checking local player and authority
  (if (Math|Boolean|ANDBoolean (Actor|ActorHasTag OtherActor "Player") (Pawn|IsLocallyControlled (Variables|/Script/Engine.Actor|GetInstigator OtherActor)) (Ability|HasAuthority OtherActor))
    (Collision|SetCollisionEnabled (Variables|Default|GetBox) "NoCollision")
    (Class|BPINetGameInstanceCommunication|ICloseSessionJoinability(Message) (Game|GetGameInstance))
    (Class|BPINETPlayerCommunication|IMoveLocalPlayer(Message) OtherActor (Transformation|GetActorLocation (Variables|Default|GetTP_Target)))
    (else
      (Development|PrintString "No player / Authority"))))

(fn ConstructionScript)