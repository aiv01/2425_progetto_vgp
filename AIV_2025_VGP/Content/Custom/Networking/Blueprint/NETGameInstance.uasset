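; Game Instance that manages online session setup through a Steam API wrapper object.
; On Init it fetches and stores the unique API instance, then de-initializes and re-initializes its online callbacks.
; A SessionCreation event requests a session through that API with a test map as travel target and a small public connection limit, then prints the request's return value.
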(event Custom|SessionCreation
  (bind _returnvalue (Class|PNetworkingInstanceSteam|RequestSessionCreation (Variables|Default|GetSteamAPI) (Utilities|Struct|MakeSessionCreationParameters "/Game/Custom/Networking/Maps/MapTest" 4 0 false true false false true true true true)))
  (Development|PrintString (Utilities|String|Append "Request Session Creation return: " (Utilities|String|ToString(Boolean) _returnvalue))))

(event EventInit
  (bind _returnvalue (Class|PNetworkingInstanceSteam|GetUniqueInstance))
  (Variables|Default|SetSteamAPI _returnvalue)
  (Class|PNetworkingInstanceSteam|DeInitializeOnlineCallbacks (Variables|Default|GetSteamAPI))
  (Class|PNetworkingInstanceSteam|InitializeOnlineCallbacks (Variables|Default|GetSteamAPI)))