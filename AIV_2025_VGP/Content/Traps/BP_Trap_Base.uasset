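; Base trap Blueprint that damages an actor when activated and provides hooks for placement and reset.
; ActivateTrap runs a box overlap query on its Box component, applies the configured damage and damage type to the hit actor, then calls ResetTrap.
; ResetTrap is empty, and OnPlaced checks the trap type enum but has no actions on its branches yet.
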(event Custom|ActivateTrap
  (bind _outhit (Class|PrimitiveComponent|BoxOverlapComponent :self (Variables|Default|GetBox)))
  (Game|Damage|ApplyDamage (.hitactor _outhit) (Variables|Default|GetDamage) 0 0 (Variables|Default|GetDamageType))
  (CallFunction|ResetTrap))

(event Custom|ResetTrap)

(event Custom|OnPlaced
  (if (not (Utilities|Enum|Equal(Enum) (Variables|Default|GetTrapType) "NewEnumerator0"))
    (if (Utilities|Enum|Equal(Enum) (Variables|Default|GetTrapType) "NewEnumerator1")
      _)))

(fn ConstructionScript)